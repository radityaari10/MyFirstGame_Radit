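; Score handler Blueprint that adds points to the player's score when an enemy dies and updates the HUD.
; On BeginPlay it binds OnEnemyDead to the enemy-death event and, after a one-second delay, caches the player pawn as BP_MyAnimationCharacter.
; Each death adds AddedScore to the character's CurrentScore, then passes the total to its player HUD widget, provided the cached character is valid.
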(event `self.ReceiveBeginPlay`
  (`|ExecutionSequence`
    (:`then_0`
      (`KismetSystemLibrary.Delay` 1.0)
      (bind _asbp_my_animation_character (cast `/Game/__Task4AnimationAndMechanic/_Blueprints/Game/BP_MyAnimationCharacter` (`GameplayStatics.GetPlayerPawn` 0)))
      (set `self.BPMyAnimationCharacter` _asbp_my_animation_character))
    (:`then_1`
      (add `self.EnemyDead` (delegate `OnEnemyDead`)))))

(event `OnEnemyDead` :!signature `self.EnemyDead`
  (params (AddedScore :type Integer))
  (bind _bpmyanimationcharacter (`self.BPMyAnimationCharacter`))
  (`/Engine/EditorBlueprintResources/StandardMacros.IsValid` (`self.BPMyAnimationCharacter`)
    (:`Is Valid`
      (bind _output_get (set `/Game/__Task4AnimationAndMechanic/_Blueprints/Game/BP_MyAnimationCharacter.CurrentScore` (+ (`/Game/__Task4AnimationAndMechanic/_Blueprints/Game/BP_MyAnimationCharacter.CurrentScore` _bpmyanimationcharacter) AddedScore) _bpmyanimationcharacter))
      (`/Game/__Task4AnimationAndMechanic/_Blueprints/UI/Player/WBP_PlayerHUD.SetScoreView` (`/Game/__Task4AnimationAndMechanic/_Blueprints/Game/BP_MyAnimationCharacter.WBPPlayerHUD` _bpmyanimationcharacter) _output_get))))

(fn `UserConstructionScript`)