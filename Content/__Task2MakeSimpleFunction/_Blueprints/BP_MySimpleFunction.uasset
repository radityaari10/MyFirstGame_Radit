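; Practice actor for an even/odd guessing game that scores the per-instance IsEvens guesses on BeginPlay.
; It creates the WBP_MySimpleFunction widget with UI-only input, then checks each guess against a random key's parity.
; CheckAnswer_Macro maintains correct and wrong streak counters, which UpdateScore uses for bonuses or penalties.
; A non-streak correct answer reuses the current ScoreEarned; turns print to screen, and the widget receives the final score.
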(event `self.ReceiveBeginPlay`
  (bind _returnvalue (`GameplayStatics.GetPlayerController` 0))
  (`|ExecutionSequence`
    (:`then_0`
      ;[1 1 1] Create Widget WBP_MySimpleFunction
      (bind _returnvalue_2 (`|CreateWidget` "/Game/__Task2MakeSimpleFunction/_Blueprints/WBP_MySimpleFunction.WBP_MySimpleFunction_C"))
      (bind _output_get (set `self.WBPMySimpleFunction` _returnvalue_2))
      (`UserWidget.AddToViewport` _output_get 0)
      (`WidgetBlueprintLibrary.SetInputMode_UIOnlyEx` _returnvalue _output_get)
      (set `PlayerController.bShowMouseCursor` true _returnvalue)
      (set `/Game/__Task2MakeSimpleFunction/_Blueprints/WBP_MySimpleFunction.BPMySimpleFunction` self (`self.WBPMySimpleFunction`)))
    (:`then_1`
      ;[1 1 1] 1. looping based on IsEvens length (editable from actor detail)
      ; 2. keyToCheck = random range (1-50)
      ; 3. modulo results of keyToCheck values compared to our guesses, Whether even or not
      (for _index (range (`KismetArrayLibrary.Array_Length` (`self.IsEvens`)))
        (`self.GenerateKeyToCheck`)
        (bind _output (`|GetArrayItem` (`self.IsEvens`) _index))
        (`KismetSystemLibrary.PrintString` (`KismetStringLibrary.Concat_StrStr` "Turn  " (`KismetStringLibrary.Conv_IntToString` (+ _index 1)) " (your guess (is even) : " (`KismetStringLibrary.Conv_BoolToString` _output) ", key to check " (`KismetStringLibrary.Conv_IntToString` (`self.keyToCheck`)) ") :"))
        (bind _iscorrectanswer (`self.CheckAnswer_Macro` _output (`self.keyToCheck`))
          (:`correct`
            _)
          (:`wrong`
            _))
        (`self.UpdateScore` _iscorrectanswer (>= (`self.StreakCorrectAnswerCounter`) 3) (>= (`self.StreakWrongAnswerCounter`) 2)))
      (`KismetSystemLibrary.PrintString` (`KismetStringLibrary.Concat_StrStr` "Your final Score : " (`KismetStringLibrary.Conv_IntToString` (`self.Score`))) true true (struct :`R` 0.063832 :`G` 1.0 :`B` 0.333052 :`A` 1.0) 10.0)
      (`/Game/__Task2MakeSimpleFunction/_Blueprints/WBP_MySimpleFunction.UpdateScoreUI` (`self.WBPMySimpleFunction`) (`self.Score`))
      (set `self.StreakCorrectAnswerCounter` 0)
      (set `self.StreakWrongAnswerCounter` 0))))

(fn `CheckAnswer`
  (params (isEven :type Boolean) (key :type Integer))
  (returns (isCorrectAnswer :type Boolean))
  (bind _iscorrectanswer (`self.CheckAnswer_Macro` isEven key)
    (:`correct`
      _)
    (:`wrong`
      _))
  (return _iscorrectanswer))

(fn `GenerateKeyToCheck`
  (returns (KeyToCheck :type Integer))
  (bind _output_get (set `self.keyToCheck` (`KismetMathLibrary.RandomIntegerInRange` 1 50)))
  (return _output_get))

(fn `UpdateScore`
  (params (isCorrectAnswer :type Boolean) (isStreakCorrectAnswer :type Boolean) (isStreakWrongAnswer :type Boolean))
  (returns (newScore :type Integer))
  (locals (ScoreEarned :type Integer :default 5))
  ;[1 1 1] < 3x benar ScoreEarned = 5;
  ; >= 3x benar ScoreEarned = 10;
  ; >= 2x salah ScoreEarned = -5;
  (if isCorrectAnswer
    (`KismetSystemLibrary.PrintString` (`KismetStringLibrary.Concat_StrStr` "your answer is correct " (`KismetStringLibrary.Conv_IntToString` (`self.StreakCorrectAnswerCounter`)) "x"))
    (if isStreakCorrectAnswer
      (set `local.ScoreEarned` 10))
    (else
      (`KismetSystemLibrary.PrintString` (`KismetStringLibrary.Concat_StrStr` "your answer is wrong " (`KismetStringLibrary.Conv_IntToString` (`self.StreakWrongAnswerCounter`)) "x"))
      (if isStreakWrongAnswer
        (set `local.ScoreEarned` -5)
        (else
          (set `local.ScoreEarned` 0)))))
  (bind _output_get (set `self.Score` (+ (`self.Score`) (`local.ScoreEarned`))))
  (`KismetSystemLibrary.PrintString` (`KismetStringLibrary.Concat_StrStr` "Score Earned : " (`KismetStringLibrary.Conv_IntToString` (`local.ScoreEarned`)) " \nYour Score : " (`KismetStringLibrary.Conv_IntToString` (`self.Score`)) " \n------------------------------ \n"))
  (return _output_get))

(fn `UserConstructionScript`)