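; Base enemy AI that patrols random nearby points, chases pawns it sees and fires a rifle within range.
; AIMoveTo callbacks loop patrol and chase, with failed chases returning to patrol.
; Rate-limited firing plays a montage and line-traces from the muzzle, sending damage through an interaction message, until the player dies.
; Incoming hits reduce health and ragdoll the mesh at zero, without stopping the AI loops.
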(event `self.ReceiveBeginPlay`
  (`KismetSystemLibrary.Delay` 0.2)
  (`self.Patrol`)
  (bind _asbp_my_animation_character (cast `/Game/__Task4AnimationAndMechanic/_Blueprints/Game/BP_MyAnimationCharacter` (`GameplayStatics.GetPlayerPawn` 0)))
  (add `/Game/__Task4AnimationAndMechanic/_Blueprints/Game/BP_MyAnimationCharacter.PlayerDead` _asbp_my_animation_character (delegate `OnPlayerDead`)))

(event `OnPlayerDead`
  (set `self.IsPlayerDead` true))

(event `/Game/_Blueprints/Interface/BPI_Interaction.OnHitObjectInteraction`
  (params (baseDamage :type "Float (double-precision)"))
  (if (!= baseDamage 0.0)
    (`GameplayStatics.ApplyDamage` self baseDamage)))

(event `self.ReceiveAnyDamage`
  (params (Damage :type "Float (single-precision)") (DamageType :type "DamageType Object Reference") (InstigatedBy :type "Controller Object Reference") (DamageCauser :type "Actor Object Reference"))
  (if (not (`self.IsDead`))
    (bind _output_get (set `self.Health` (- (`self.Health`) Damage)))
    (`KismetSystemLibrary.PrintString` (`KismetStringLibrary.Concat_StrStr` (`KismetSystemLibrary.GetDisplayName` self) "(Health) : " (`KismetStringLibrary.Conv_DoubleToString` _output_get)))
    (if (<= (`self.Health`) 0.0)
      (`PrimitiveComponent.SetSimulatePhysics` (`self.Mesh`) true)
      (set `self.IsDead` true))))

(event `Patrol`
  (`|AIMoveTo` self (`NavigationSystemV1.K2_GetRandomReachablePointInRadius` (`self.K2_GetActorLocation`) 300.0 null null) null
    (:`OnSuccess`
      _)
    (:`OnFail`
      _))
  (`self.Patrol`))

(event `ChasePlayer`
  (params (TargetActor :type "Actor Object Reference"))
  (`|AIMoveTo` self (0.0 0.0 0.0) TargetActor 300.0
    (:`OnSuccess`
      (`self.Fire`)
      (`self.ChasePlayer` TargetActor))
    (:`OnFail`
      (`self.Patrol`))))

(event `self.PawnSensing.OnSeePawn`
  (params (Pawn :type "Pawn Object Reference"))
  (`self.ChasePlayer` Pawn))

(event `Fire`
  (bind _returnvalue_location (`KismetMathLibrary.BreakTransform` (`SceneComponent.GetSocketTransform` (`self.Rifle`) "Muzzle" "RTS_World")))
  (if (not (`self.IsPlayerDead`))
    (`/Engine/EditorBlueprintResources/StandardMacros.DoOnce` false :!label _label
      (:`Completed`
        (`|ExecutionSequence`
          (:`then_0`
            (`|PlayMontage` (`self.Mesh`) "/Game/Characters/MyAvatar/RTGAnimations/RPM_Fire_Rifle_Ironsights_Montage.RPM_Fire_Rifle_Ironsights_Montage"
              (:`then`
                (bind _outhit (`KismetSystemLibrary.LineTraceSingle` :`Start` _returnvalue_location :`End` (+ _returnvalue_location (* (`SceneComponent.GetRightVector` (`self.Mesh`)) 3000.0)) :`TraceChannel` "TraceTypeQuery1" :`DrawDebugType` "ForDuration"))
                (message `/Game/_Blueprints/Interface/BPI_Interaction.OnHitObjectInteraction` (`.HitActor` (`GameplayStatics.BreakHitResult` _outhit)) 20.0))))
          (:`then_1`
            (`KismetSystemLibrary.Delay` 0.24)
            (goto _label :!via `Reset`)))))))

(fn `UserConstructionScript`)