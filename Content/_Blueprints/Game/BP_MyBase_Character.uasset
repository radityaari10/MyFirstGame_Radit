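; Base character Blueprint providing shared rifle firing, damage and death, with empty hooks for children to extend.
; Fire uses a DoOnce reset by a short delay to throttle shots, plays a montage and line-traces from a rifle socket with debug drawing.
; Hit actors receive an interaction message, which this class converts into ApplyDamage on itself.
; Damage updates health and the health bar widget, ragdolling the mesh and flagging death at zero.
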(event `self.ReceiveBeginPlay`
  (bind _asbp_my_third_person_game_instance (cast `/Game/_Blueprints/Game/BP_MyThirdPerson_GameInstance` (`GameplayStatics.GetGameInstance`)))
  (set `self.BPMyThirdPersonGameInstance` _asbp_my_third_person_game_instance))

(event `/Game/_Blueprints/Interface/BPI_Interaction.OnHitObjectInteraction`
  (params (baseDamage :type "Float (double-precision)"))
  (if (!= baseDamage 0.0)
    (`GameplayStatics.ApplyDamage` self baseDamage)))

(event `self.ReceiveAnyDamage`
  (params (Damage :type "Float (single-precision)") (DamageType :type "DamageType Object Reference") (InstigatedBy :type "Controller Object Reference") (DamageCauser :type "Actor Object Reference"))
  (`self.AnyDamageFromOther` (- (`self.CurrentHealth`) Damage)))

(event `/Game/_Blueprints/Interface/Character/BPI_MyCharacter.Fire`
  (params (MontageToPlay :type "AnimMontage Object Reference") (RifleInSocketName :type Name) (EndVector :type "Vector Structure"))
  (bind _returnvalue_location (`KismetMathLibrary.BreakTransform` (`SceneComponent.GetSocketTransform` (`self.Rifle`) RifleInSocketName "RTS_World")))
  (`/Engine/EditorBlueprintResources/StandardMacros.DoOnce` false :!label _label
    (:`Completed`
      (`|ExecutionSequence`
        (:`then_0`
          (`|PlayMontage` (`self.Mesh`) MontageToPlay
            (:`then`
              (`self.FireAfterAnimation`)
              (bind _outhit (`KismetSystemLibrary.LineTraceSingle` :`Start` _returnvalue_location :`End` (+ _returnvalue_location (* EndVector 3000.0)) :`TraceChannel` "TraceTypeQuery1" :`DrawDebugType` "ForDuration"))
              (message `/Game/_Blueprints/Interface/BPI_Interaction.OnHitObjectInteraction` (`.HitActor` (`GameplayStatics.BreakHitResult` _outhit)) 20.0))))
        (:`then_1`
          (`KismetSystemLibrary.Delay` 0.24)
          (goto _label :!via `Reset`))))))

(event `/Game/_Blueprints/Interface/Character/BPI_MyCharacter.AnyDamageFromOther`
  (params (CurrentHealth :type "Float (double-precision)"))
  (if (not (`self.IsDead`))
    (set `self.CurrentHealth` CurrentHealth)
    (`/Game/__Task4AnimationAndMechanic/_Blueprints/UI/Player/WBP_HealthBar.SetHealtBarView` (`self.WBPHealthBar`) (`self.CurrentHealth`) (`self.MaxHealth`))
    (if (<= (`self.CurrentHealth`) 0.0)
      (`self.AnyDamageApplyDeath`)
      (else
        (`self.AnyDamageApplyAlive`)))))

(event `/Game/_Blueprints/Interface/Character/BPI_MyCharacter.AnyDamageApplyDeath`
  (`PrimitiveComponent.SetSimulatePhysics` (`self.Mesh`) true)
  (set `self.IsDead` true))

(event `/Game/_Blueprints/Interface/Character/BPI_MyCharacter.AnyDamageApplyAlive`)

(event `/Game/_Blueprints/Interface/Character/BPI_MyCharacter.FireAfterAnimation`)

(fn `UserConstructionScript`)